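; Game mode that runs the start and death flow for a ship game, with audio fades.
; BeginPlay resets lives and score in BP_GI, disables ship input, lowers audio volume and pitch parameters to initial values and shows the start menu.
; Jugar marks the game started, ramps volume then pitch through chained timelines, then enables input and swaps to the HUD.
; Morir plays similar timelines in reverse, volume before pitch.
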(event `self.ReceiveBeginPlay`
  (bind _returnvalue (`GameplayStatics.GetPlayerController` 0))
  (bind _as_bp_gi (`self.As BP GI`))
  (bind _asbp_gi (cast `/Game/BP/BP_GI` (`GameplayStatics.GetGameInstance`)))
  (set `self.As BP GI` _asbp_gi)
  (set `/Game/BP/BP_GI.VidaNave` 3 _as_bp_gi)
  (set `/Game/BP/BP_GI.Puntos` 0 _as_bp_gi)
  (bind _returnvalue_2 (`GameplayStatics.GetActorOfClass` (`self.DefaultPawnClass`)))
  (bind _output_get (set `self.Pawn Nave` _returnvalue_2))
  (`self.DisableInput` _output_get (`GameplayStatics.GetPlayerController` 0))
  (`AudioComponent.SetFloatParameter` (`self.Audio`) "Pitch Multi" (`self.Pitch Ini`))
  (`AudioComponent.SetFloatParameter` (`self.Audio`) "Volumen" (`self.Volumen`))
  (bind _returnvalue_3 (`|CreateWidget` "/Game/Widgets/WBP_Inicio.WBP_Inicio_C" (`GameplayStatics.GetPlayerController` 0)))
  (bind _output_get_2 (set `self.Widget Ref` _returnvalue_3))
  (`UserWidget.AddToViewport` _output_get_2 0)
  (set `PlayerController.bShowMouseCursor` true _returnvalue)
  (`WidgetBlueprintLibrary.SetInputMode_GameAndUIEx` _returnvalue (`self.Widget Ref`)))

(event `Jugar`
  (bind _returnvalue (`GameplayStatics.GetPlayerController` 0))
  (bind _returnvalue_2 (`GameplayStatics.GetPlayerController` 0))
  (set `/Game/BP/BP_GI.Started` true (`self.As BP GI`))
  (set `PlayerController.bShowMouseCursor` false _returnvalue_2)
  (`WidgetBlueprintLibrary.SetInputMode_GameOnly` _returnvalue_2)
  (bind (_direction _lerp) (`Timeline|Timeline` :!via `PlayFromStart`)
    (:`Update`
      (`AudioComponent.SetFloatParameter` (`self.Audio`) "Volumen" (`KismetMathLibrary.MapRangeClamped` _lerp 0.0 1.0 (`self.Volumen`) 1.0)))
    (:`Finished`
      (bind (_direction_2 _lerp_2) (`Timeline|Timeline_0` :!via `PlayFromStart`)
        (:`Update`
          (`AudioComponent.SetFloatParameter` (`self.Audio`) "Pitch Multi" (`KismetMathLibrary.MapRangeClamped` _lerp_2 0.0 1.0 (`self.Pitch Ini`) 1.0)))
        (:`Finished`
          (`self.EnableInput` (`self.Pawn Nave`) _returnvalue)
          (`Widget.RemoveFromParent` (`self.Widget Ref`))
          (bind _returnvalue_3 (`|CreateWidget` "/Game/Widgets/WBP_InGame.WBP_InGame_C" _returnvalue))
          (`UserWidget.AddToPlayerScreen` _returnvalue_3 0))))))

(event `Morir`
  (bind (_direction _lerp) (`Timeline|Timeline_1` :!via `ReverseFromEnd`)
    (:`Update`
      (`AudioComponent.SetFloatParameter` (`self.Audio`) "Volumen" (`KismetMathLibrary.MapRangeClamped` _lerp 0.0 1.0 (`self.Volumen`) 1.0)))
    (:`Finished`
      (bind (_direction_2 _lerp_2) (`Timeline|Timeline_2` :!via `ReverseFromEnd`)
        (:`Update`
          (`AudioComponent.SetFloatParameter` (`self.Audio`) "Pitch Multi" (`KismetMathLibrary.MapRangeClamped` _lerp_2 0.0 1.0 (`self.Pitch Ini`) 1.0)))))))

(fn `UserConstructionScript`)