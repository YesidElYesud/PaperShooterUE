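; BP_ControlSound drives an audio component's volume and pitch parameters in response to play (Jugar) and death (Morir) events.
; BeginPlay applies the initial Volumen and PitchIni values.
; Jugar runs two chained timelines, blending volume to 1.0 and then pitch to 1.0.
; Morir plays a separate timeline pair in reverse, returning volume and then pitch to their initial values.
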(event `self.ReceiveBeginPlay`
  (`AudioComponent.SetFloatParameter` (`self.Audio`) "Pitch Multi" (`self.Pitch Ini`))
  (`AudioComponent.SetFloatParameter` (`self.Audio`) "Volumen" (`self.Volumen`)))

(event `Jugar`
  (bind (_direction _lerp) (`Timeline|Timeline` :!via `PlayFromStart`)
    (:`Update`
      (`AudioComponent.SetFloatParameter` (`self.Audio`) "Volumen" (`KismetMathLibrary.MapRangeClamped` _lerp 0.0 1.0 (`self.Volumen`) 1.0)))
    (:`Finished`
      (bind (_direction_2 _lerp_2) (`Timeline|Timeline_1` :!via `PlayFromStart`)
        (:`Update`
          (`AudioComponent.SetFloatParameter` (`self.Audio`) "Pitch Multi" (`KismetMathLibrary.MapRangeClamped` _lerp_2 0.0 1.0 (`self.Pitch Ini`) 1.0)))))))

(event `Morir`
  (bind (_direction _lerp) (`Timeline|Timeline_0` :!via `ReverseFromEnd`)
    (:`Update`
      (`AudioComponent.SetFloatParameter` (`self.Audio`) "Volumen" (`KismetMathLibrary.MapRangeClamped` _lerp 0.0 1.0 (`self.Volumen`) 1.0)))
    (:`Finished`
      (bind (_direction_2 _lerp_2) (`Timeline|Timeline_2` :!via `ReverseFromEnd`)
        (:`Update`
          (`AudioComponent.SetFloatParameter` (`self.Audio`) "Pitch Multi" (`KismetMathLibrary.MapRangeClamped` _lerp_2 0.0 1.0 (`self.Pitch Ini`) 1.0)))))))

(fn `UserConstructionScript`)